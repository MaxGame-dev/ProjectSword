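; BP_EventBase is an event object, apparently a base Blueprint, whose static mesh look reflects its event type.
; On BeginPlay it checks EventType and sets the mesh's first material slot to the recovery, gate or save material.
; Other types keep the default material, and the file holds no further event behavior.
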(event `self.ReceiveBeginPlay`
  (if (== (`self.EventType`) 1)
    (`PrimitiveComponent.SetMaterial` (`self.StaticMesh`) 0 "/Game/Project/Assets/Materials/M_EventRecovery.M_EventRecovery")
    (elif (== (`self.EventType`) 2)
      (`PrimitiveComponent.SetMaterial` (`self.StaticMesh`) 0 "/Game/Project/Assets/Materials/M_Gate.M_Gate")
      (elif (== (`self.EventType`) 3)
        (`PrimitiveComponent.SetMaterial` (`self.StaticMesh`) 0 "/Game/Project/Assets/Materials/M_EventSave.M_EventSave")))))

(fn `UserConstructionScript`)