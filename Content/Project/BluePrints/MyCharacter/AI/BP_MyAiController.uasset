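; AI controller for AI-driven BP_MyCharacter pawns that hunts human-controlled players.
; On BeginPlay it sets up its blackboard and runs its behavior tree.
; AI Perception updates feed SetTargetPlayer, which, while the pawn has Hp left, picks out non-AI characters.
; It writes the first stimulus's sensed state to the IsSearch key and sets or clears TargetPlayer accordingly.
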(event `self.ReceiveBeginPlay`
  (`self.UseBlackboard` "/Game/Project/BluePrints/MyCharacter/AI/BB_MyAiController.BB_MyAiController")
  (`self.RunBehaviorTree` "/Game/Project/BluePrints/MyCharacter/AI/BT_MyAiController.BT_MyAiController"))

(event `self.AIPerception.OnPerceptionUpdated`
  (params (UpdatedActors :type "Array of Actor Object Reference (by ref)"))
  (`self.SetTargetPlayer` UpdatedActors))

(fn `SetTargetPlayer`
  (params (`UpdatedActors[` :type "Array of Actor Object Reference"))
  (bind _asbp_my_character (cast `/Game/Project/BluePrints/MyCharacter/BP_MyCharacter` (`self.K2_GetPawn`) :!pure true))
  (`/Engine/EditorBlueprintResources/StandardMacros.IsValid` _asbp_my_character
    (:`Is Valid`
      (if (> (`/Game/Project/BluePrints/MyCharacter/BP_MyCharacter.Hp` _asbp_my_character) 0)
        (for _array_element `UpdatedActors[`
          (bind _info (`AIPerceptionComponent.GetActorsPerception` (`self.AIPerception`) _array_element))
          (bind (_target _lastsensedstimuli) (break `ActorPerceptionBlueprintInfo` _info))
          (bind _asbp_my_character_2 (cast `/Game/Project/BluePrints/MyCharacter/BP_MyCharacter` _target :!pure true))
          (`/Engine/EditorBlueprintResources/StandardMacros.IsValid` _asbp_my_character_2
            (:`Is Valid`
              (if (not (`/Game/Project/BluePrints/MyCharacter/BP_MyCharacter.IsAi` _asbp_my_character_2))
                (set `self.TargetActor` _target)
                (bind (_age _expirationage _strength _stimuluslocation _receiverlocation _tag _bsuccessfullysensed) (break `AIStimulus` (`|GetArrayItem` _lastsensedstimuli)))
                (`BlackboardComponent.SetValueAsBool` (`AIBlueprintHelperLibrary.GetBlackboard` null) "IsSearch" _bsuccessfullysensed)
                (if _bsuccessfullysensed
                  (`BlackboardComponent.SetValueAsObject` (`AIBlueprintHelperLibrary.GetBlackboard` null) "TargetPlayer" (`self.TargetActor`))
                  (else
                    (`BlackboardComponent.SetValueAsObject` (`AIBlueprintHelperLibrary.GetBlackboard` null) "TargetPlayer" null)))))))))))

(fn `UserConstructionScript`)