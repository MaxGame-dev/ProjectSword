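; Anim notify state that blocks attack and/or dodge input on BP_MyCharacter during a window of an animation.
; Begin and every tick set the owner's IsEnableAttack and IsEnableDodge to false, as selected by the Attack and Dodge flags.
; End sets the selected flags back to true without saving their prior values.
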(fn `Received_NotifyBegin`
  (params (MeshComp :type "SkeletalMeshComponent Object Reference") (Animation :type "AnimSequenceBase Object Reference") (TotalDuration :type "Float (single-precision)") (EventReference :type "AnimNotifyEventReference Structure (by ref)"))
  (returns (ReturnValue :type Boolean))
  (bind _asbp_my_character (cast `/Game/Project/BluePrints/Characters/BP_MyCharacter` (`ActorComponent.GetOwner` MeshComp) :!pure true))
  (`/Engine/EditorBlueprintResources/StandardMacros.IsValid` _asbp_my_character
    (:`Is Valid`
      (`|ExecutionSequence`
        (:`then_0`
          (if (`self.Attack`)
            (set `/Game/Project/BluePrints/Characters/BP_MyCharacter.IsEnableAttack` false _asbp_my_character)))
        (:`then_1`
          (if (`self.Dodge`)
            (set `/Game/Project/BluePrints/Characters/BP_MyCharacter.IsEnableDodge` false _asbp_my_character)
            (return false)))))))

(fn `Received_NotifyEnd`
  (params (MeshComp :type "SkeletalMeshComponent Object Reference") (Animation :type "AnimSequenceBase Object Reference") (EventReference :type "AnimNotifyEventReference Structure (by ref)"))
  (returns (ReturnValue :type Boolean))
  (bind _asbp_my_character (cast `/Game/Project/BluePrints/Characters/BP_MyCharacter` (`ActorComponent.GetOwner` MeshComp) :!pure true))
  (`/Engine/EditorBlueprintResources/StandardMacros.IsValid` _asbp_my_character
    (:`Is Valid`
      (`|ExecutionSequence`
        (:`then_0`
          (if (`self.Attack`)
            (set `/Game/Project/BluePrints/Characters/BP_MyCharacter.IsEnableAttack` true _asbp_my_character)))
        (:`then_1`
          (if (`self.Dodge`)
            (set `/Game/Project/BluePrints/Characters/BP_MyCharacter.IsEnableDodge` true _asbp_my_character)
            (return false)))))))

(fn `Received_NotifyTick`
  (params (MeshComp :type "SkeletalMeshComponent Object Reference") (Animation :type "AnimSequenceBase Object Reference") (FrameDeltaTime :type "Float (single-precision)") (EventReference :type "AnimNotifyEventReference Structure (by ref)"))
  (returns (ReturnValue :type Boolean))
  (bind _asbp_my_character (cast `/Game/Project/BluePrints/Characters/BP_MyCharacter` (`ActorComponent.GetOwner` MeshComp) :!pure true))
  (`/Engine/EditorBlueprintResources/StandardMacros.IsValid` _asbp_my_character
    (:`Is Valid`
      (`|ExecutionSequence`
        (:`then_0`
          (if (`self.Attack`)
            (set `/Game/Project/BluePrints/Characters/BP_MyCharacter.IsEnableAttack` false _asbp_my_character)))
        (:`then_1`
          (if (`self.Dodge`)
            (set `/Game/Project/BluePrints/Characters/BP_MyCharacter.IsEnableDodge` false _asbp_my_character)
            (return false)))))))