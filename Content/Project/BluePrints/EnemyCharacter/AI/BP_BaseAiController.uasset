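; BP_BaseAiController is the base AI controller for enemy BP_MyCharacter pawns, detecting human players and locking onto them.
; On BeginPlay or RespawnAi, it caches its pawn and runs the behavior tree from that character type's DT_CharacterData row on BB_BaseAiController.
; While the pawn is alive, perception updates set IsSearch from the first stimulus.
; Sensing sets TargetPlayer and starts lock-on following; losing it releases lock-on without clearing TargetPlayer.
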(event `self.ReceiveBeginPlay`
  (bind _asbp_my_character (cast `/Game/Project/BluePrints/MyCharacter/BP_MyCharacter` (`self.K2_GetPawn`) :!pure true))
  (`/Engine/EditorBlueprintResources/StandardMacros.IsValid` _asbp_my_character :!label _label
    (:`Is Valid`
      (bind _output_get (set `self.MyCharacter` _asbp_my_character))
      (bind _returnvalue (`|GetDataTableRow` "/Game/Project/BluePrints/DataTables/DT_CharacterData.DT_CharacterData" (`/Game/Project/BluePrints/MyCharacter/BP_MyCharacter.CharacterTypeName` _output_get))
        (:`then`
          (`self.UseBlackboard` "/Game/Project/BluePrints/EnemyCharacter/AI/BB_BaseAiController.BB_BaseAiController")
          (`self.RunBehaviorTree` (`.BTAsset_104_86CE89EF42DB07304784C3B09485C5E0` (break `/Game/Project/BluePrints/DataTables/ST_CharacterData` _returnvalue))))))))

(event `RespawnAi`
  (goto _label))

(event `self.AIPerception.OnPerceptionUpdated`
  (params (UpdatedActors :type "Array of Actor Object Reference (by ref)"))
  (`self.SetTargetPlayer` UpdatedActors))

(fn `SetTargetPlayer`
  (params (UpdatedActors :type "Array of Actor Object Reference"))
  (bind _mycharacter (`self.MyCharacter`))
  (bind _mycharacter_2 (`self.MyCharacter`))
  (bind _mycharacter_3 (`self.MyCharacter`))
  (`/Engine/EditorBlueprintResources/StandardMacros.IsValid` _mycharacter
    (:`Is Valid`
      (if (> (`/Game/Project/BluePrints/MyCharacter/BP_MyCharacter.Hp` _mycharacter) 0.0)
        (for _array_element UpdatedActors
          (bind _info (`AIPerceptionComponent.GetActorsPerception` (`self.AIPerception`) _array_element))
          (bind (_target _lastsensedstimuli) (break `ActorPerceptionBlueprintInfo` _info))
          (bind _asbp_my_character (cast `/Game/Project/BluePrints/MyCharacter/BP_MyCharacter` _target :!pure true))
          (`/Engine/EditorBlueprintResources/StandardMacros.IsValid` _asbp_my_character
            (:`Is Valid`
              (if (not (`/Game/Project/BluePrints/MyCharacter/BP_MyCharacter.IsAi` _asbp_my_character))
                (set `self.TargetActor` _target)
                (bind (_age _expirationage _strength _stimuluslocation _receiverlocation _tag _bsuccessfullysensed) (break `AIStimulus` (`|GetArrayItem` _lastsensedstimuli)))
                (`BlackboardComponent.SetValueAsBool` (`AIBlueprintHelperLibrary.GetBlackboard` null) "IsSearch" _bsuccessfullysensed)
                (if _bsuccessfullysensed
                  (`BlackboardComponent.SetValueAsObject` (`AIBlueprintHelperLibrary.GetBlackboard` null) "TargetPlayer" (`self.TargetActor`))
                  (`/Game/Project/BluePrints/MyCharacter/BP_MyCharacter.SetLockOn` _mycharacter_2 true (`self.TargetActor`))
                  (`/Game/Project/BluePrints/MyCharacter/BP_MyCharacter.SetTargetIsLockedOn` _mycharacter_2 true)
                  (`/Game/Project/BluePrints/MyCharacter/BP_MyCharacter.AiStartFollowLockOnPlayer` _mycharacter_2)
                  (else
                    (`/Game/Project/BluePrints/MyCharacter/BP_MyCharacter.SetTargetIsLockedOn` _mycharacter_3 false)
                    (`/Game/Project/BluePrints/MyCharacter/BP_MyCharacter.SetLockOn` _mycharacter_3 false null)))))))))))

(fn `UserConstructionScript`)