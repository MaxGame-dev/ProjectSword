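; Base AI controller for enemy characters that detects and locks onto human-controlled players.
; On BeginPlay it starts its Blackboard and Behavior Tree and caches the possessed BP_EnemyBase.
; Perception updates, while the enemy is alive, write the IsSearch and TargetPlayer keys from the first stimulus of each non-AI BP_MyCharacter.
; Successful sensing turns on the enemy's lock-on and follow; losing it clears the target and lock-on.
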(event `self.ReceiveBeginPlay`
  (bind _asbp_enemy_base (cast `/Game/Project/BluePrints/EnemyCharacter/BP_EnemyBase` (`self.K2_GetPawn`) :!pure true))
  (`self.UseBlackboard` "/Game/Project/BluePrints/EnemyCharacter/AI/BB_EnemyBaseAiController.BB_EnemyBaseAiController")
  (`self.RunBehaviorTree` "/Game/Project/BluePrints/EnemyCharacter/AI/BT_EnemyBaseAiController.BT_EnemyBaseAiController")
  (`/Engine/EditorBlueprintResources/StandardMacros.IsValid` _asbp_enemy_base
    (:`Is Valid`
      (set `self.EnemyBase` _asbp_enemy_base))))

(event `self.AIPerception.OnPerceptionUpdated`
  (params (UpdatedActors :type "Array of Actor Object Reference (by ref)"))
  (`self.SetTargetPlayer` UpdatedActors))

(fn `SetTargetPlayer`
  (params (UpdatedActors :type "Array of Actor Object Reference"))
  (bind _enemybase (`self.EnemyBase`))
  (if (> (`/Game/Project/BluePrints/MyCharacter/BP_MyCharacter.Hp` (`self.EnemyBase`)) 0)
    (for _array_element UpdatedActors
      (bind _info (`AIPerceptionComponent.GetActorsPerception` (`self.AIPerception`) _array_element))
      (bind (_target _lastsensedstimuli) (break `ActorPerceptionBlueprintInfo` _info))
      (bind _asbp_my_character (cast `/Game/Project/BluePrints/MyCharacter/BP_MyCharacter` _target :!pure true))
      (`/Engine/EditorBlueprintResources/StandardMacros.IsValid` _asbp_my_character
        (:`Is Valid`
          (if (not (`/Game/Project/BluePrints/MyCharacter/BP_MyCharacter.IsAi` _asbp_my_character))
            (set `self.TargetActor` _target)
            (bind (_age _expirationage _strength _stimuluslocation _receiverlocation _tag _bsuccessfullysensed) (break `AIStimulus` (`|GetArrayItem` _lastsensedstimuli)))
            (`BlackboardComponent.SetValueAsBool` (`AIBlueprintHelperLibrary.GetBlackboard` null) "IsSearch" _bsuccessfullysensed)
            (if _bsuccessfullysensed
              (`BlackboardComponent.SetValueAsObject` (`AIBlueprintHelperLibrary.GetBlackboard` null) "TargetPlayer" (`self.TargetActor`))
              (`/Game/Project/BluePrints/MyCharacter/BP_MyCharacter.SetLockOn` _enemybase true (`self.TargetActor`))
              (`/Game/Project/BluePrints/MyCharacter/BP_MyCharacter.AiStartFollowLockOnPlayer` _enemybase)
              (else
                (`BlackboardComponent.SetValueAsObject` (`AIBlueprintHelperLibrary.GetBlackboard` null) "TargetPlayer" null)
                (`/Game/Project/BluePrints/MyCharacter/BP_MyCharacter.SetLockOn` (`self.EnemyBase`) false null)))))))))

(fn `UserConstructionScript`)