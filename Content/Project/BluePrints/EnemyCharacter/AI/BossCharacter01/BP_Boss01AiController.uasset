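; AI controller for the first boss character that starts its behavior tree and picks the player as combat target.
; On perception updates while the boss is alive, it filters for non-AI player characters and writes search state and target to the blackboard.
; Sensing a player also locks the boss onto them and starts follow behavior; losing sight clears the target and lock-on.
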(event `self.ReceiveBeginPlay`
  (bind _asbp_boss_character_01 (cast `/Game/Project/BluePrints/EnemyCharacter/BossCharacter01/BP_BossCharacter01` (`self.K2_GetPawn`) :!pure true))
  (`self.UseBlackboard` "/Game/Project/BluePrints/EnemyCharacter/AI/BossCharacter01/BB_Boss01AiController.BB_Boss01AiController")
  (`self.RunBehaviorTree` "/Game/Project/BluePrints/EnemyCharacter/AI/BossCharacter01/BT_Boss01AiController.BT_Boss01AiController")
  (`/Engine/EditorBlueprintResources/StandardMacros.IsValid` _asbp_boss_character_01
    (:`Is Valid`
      (set `self.BossCharacter` _asbp_boss_character_01))))

(event `self.AIPerception.OnPerceptionUpdated`
  (params (UpdatedActors :type "Array of Actor Object Reference (by ref)"))
  (`self.SetTargetPlayer` UpdatedActors))

(fn `SetTargetPlayer`
  (params (UpdatedActors :type "Array of Actor Object Reference"))
  (bind _bosscharacter (`self.BossCharacter`))
  (if (> (`/Game/Project/BluePrints/MyCharacter/BP_MyCharacter.Hp` (`self.BossCharacter`)) 0)
    (for _array_element UpdatedActors
      (bind _info (`AIPerceptionComponent.GetActorsPerception` (`self.AIPerception`) _array_element))
      (bind (_target _lastsensedstimuli) (break `ActorPerceptionBlueprintInfo` _info))
      (bind _asbp_my_character (cast `/Game/Project/BluePrints/MyCharacter/BP_MyCharacter` _target :!pure true))
      (`/Engine/EditorBlueprintResources/StandardMacros.IsValid` _asbp_my_character
        (:`Is Valid`
          (if (not (`/Game/Project/BluePrints/MyCharacter/BP_MyCharacter.IsAi` _asbp_my_character))
            (set `self.TargetActor` _target)
            (bind (_age _expirationage _strength _stimuluslocation _receiverlocation _tag _bsuccessfullysensed) (break `AIStimulus` (`|GetArrayItem` _lastsensedstimuli)))
            (`BlackboardComponent.SetValueAsBool` (`AIBlueprintHelperLibrary.GetBlackboard` null) "IsSearch" _bsuccessfullysensed)
            (if _bsuccessfullysensed
              (`BlackboardComponent.SetValueAsObject` (`AIBlueprintHelperLibrary.GetBlackboard` null) "TargetPlayer" (`self.TargetActor`))
              (`/Game/Project/BluePrints/MyCharacter/BP_MyCharacter.SetLockOn` _bosscharacter true (`self.TargetActor`))
              (`/Game/Project/BluePrints/MyCharacter/BP_MyCharacter.AiStartFollowLockOnPlayer` _bosscharacter)
              (else
                (`BlackboardComponent.SetValueAsObject` (`AIBlueprintHelperLibrary.GetBlackboard` null) "TargetPlayer" null)
                (`/Game/Project/BluePrints/MyCharacter/BP_MyCharacter.SetLockOn` (`self.BossCharacter`) false null)))))))))

(fn `UserConstructionScript`)